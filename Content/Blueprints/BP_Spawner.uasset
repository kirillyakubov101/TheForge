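; BP_Spawner is an actor that spawns waves of random enemies at three spawn points for BP_FirstPersonGameMode.
; On BeginPlay it collects the points and binds to the game mode's NewWave event, which resets the count.
; A Delay-based loop calls SpawnEnemy each second, picking a random class and point, until MaxSpawn is reached.
; SpawnProcess runs the same loop after an initial delay, but nothing in this graph calls it.
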(event Custom|NewWaveEvent
  (Variables|Default|SetSpawnCount 0)
  (CallFunction|SpawnEnemy :!label _label)
  (Utilities|FlowControl|Delay 1.0)
  (if (not (>= (Variables|Default|GetSpawnCount) (Variables|/Game/Blueprints/BP_FirstPersonGameMode.BP_FirstPersonGameMode_C|GetMaxSpawn (Variables|Default|GetGameMode))))
    (goto _label)))

(event EventBeginPlay
  (bind _spawnarray (Variables|Default|GetSpawnArray))
  (Utilities|Array|Add _spawnarray (Variables|Default|GetSpawn_1))
  (Utilities|Array|Add _spawnarray (Variables|Default|GetSpawn_2))
  (Utilities|Array|Add _spawnarray (Variables|Default|GetSpawn_3))
  (bind _asbp_first_person_game_mode (Utilities|Casting|CastToBP_FirstPersonGameMode (Game|GetGameMode)))
  (Variables|Default|SetGameMode _asbp_first_person_game_mode)
  (EventDispatchers|BindEventtoNewWave (Variables|Default|GetGameMode) (delegate Custom|NewWaveEvent)))

(event EventSpawnProcess
  (Utilities|FlowControl|Delay 2.0)
  (CallFunction|SpawnEnemy :!label _label)
  (Utilities|FlowControl|Delay 1.0)
  (if (not (>= (Variables|Default|GetSpawnCount) (Variables|/Game/Blueprints/BP_FirstPersonGameMode.BP_FirstPersonGameMode_C|GetMaxSpawn (Variables|Default|GetGameMode))))
    (goto _label)))

(fn ConstructionScript)

(fn SpawnEnemy
  (bind _spawnarray (Variables|Default|GetSpawnArray))
  (bind _outitem (Utilities|Array|Random _spawnarray))
  (Utilities|IsValid _outitem
    (:Is%20Valid
      (Game|SpawnActorfromClass (.OutItem (Utilities|Array|Random (Variables|Default|GetEnemiesList))) (Transformation|GetWorldTransform _outitem) "Undefined" 0 0)
      (Math|Integer|IncrementInt (Variables|Default|GetSpawnCount)))))