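; BP_HitpointsCrate is a health pickup chest that heals the BP_MyFPS player on contact.
; A sphere overlap calls HealPLayer on the player, then DisableHealingChest hides the chest and its optional SpotLight and turns off the sphere's collision.
; EnableHealingChest reverses this to make the pickup available again, though nothing in this Blueprint calls it.
; The chest mesh's own collision is switched off at BeginPlay.
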(event OnComponentBeginOverlap(Sphere)
  (params (OverlappedComponent :type Primitive%20Component%20Object%20Reference) (OtherActor :type Actor%20Object%20Reference) (OtherComp :type Primitive%20Component%20Object%20Reference) (OtherBodyIndex :type Integer) (bFromSweep :type Boolean) (SweepResult :type Hit%20Result%20Structure%20%28by%20ref%29))
  (bind _asbp_my_fps (Utilities|Casting|CastToBP_MyFPS OtherActor))
  (Default|HealPLayer _asbp_my_fps)
  (CallFunction|DisableHealingChest))

(event EventBeginPlay
  (Collision|SetCollisionEnabled (Variables|Default|GetChest) "NoCollision"))

(fn ConstructionScript)

(fn EnableHealingChest
  (bind _spotlight (Variables|Default|GetSpotLight))
  (Rendering|SetVisibility (Variables|Default|GetChest) true false)
  (Collision|SetCollisionEnabled (Variables|Default|GetSphere) "QueryOnly")
  (Utilities|IsValid _spotlight
    (:Is%20Valid
      (Rendering|SetVisibility (Variables|/Script/Engine.Light|GetLightComponent _spotlight) true false))))

(fn DisableHealingChest
  (bind _spotlight (Variables|Default|GetSpotLight))
  (Rendering|SetVisibility (Variables|Default|GetChest) false false)
  (Collision|SetCollisionEnabled (Variables|Default|GetSphere) "NoCollision")
  (Utilities|IsValid _spotlight
    (:Is%20Valid
      (Rendering|SetVisibility (Variables|/Script/Engine.Light|GetLightComponent _spotlight) false false))))