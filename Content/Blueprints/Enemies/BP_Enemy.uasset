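; BP_Enemy is an AI-driven enemy with sword and grenade attacks, entering as a physics-simulated capsule.
; Its first hit disables physics, plays an intro montage, then starts BP_AI on completion.
; Damage spawns floating text and reduces health; death notifies the game mode, spawns smoke and destroys it.
; Helper functions play attack montages and launch projectiles toward the player; DamagePlayer only plays sword sounds, its damage nodes being unconnected.
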(event OnComponentHit(CapsuleComponent)
  (params (HitComponent :type Primitive%20Component%20Object%20Reference) (OtherActor :type Actor%20Object%20Reference) (OtherComp :type Primitive%20Component%20Object%20Reference) (NormalImpulse :type Vector :default "0, 0, 0") (Hit :type Hit%20Result%20Structure%20%28by%20ref%29))
  (Utilities|FlowControl|DoOnce false
    (:Completed
      (Physics|SetSimulatePhysics (Variables|Default|GetCapsuleComponent) false)
      (Animation|Montage|PlayMontage (Variables|Character|GetMesh) "/Game/Blueprints/Enemies/AM_Intro.AM_Intro"
        (:OnCompleted
          (bind _asbp_ai (Utilities|Casting|CastToBP_AI (AI|GetAIController self)))
          (Default|RunAI _asbp_ai))))))

(event EventOnDamageEvent
  (params (damage :type Float%20%28single-precision%29))
  (Game|SpawnActorfromClass "/Game/Blueprints/Enemies/BP_DamageText.BP_DamageText_C" (Transformation|GetActorTransform) "Undefined" 0 damage 0)
  (Variables|Default|SetHealth (- (Variables|Default|GetHealth) damage))
  (if (<= (Variables|Default|GetHealth) 0.0)
    (bind _asbp_first_person_game_mode (Utilities|Casting|CastToBP_FirstPersonGameMode (Game|GetGameMode)))
    (Default|OnEnemyKilled _asbp_first_person_game_mode)
    (Effects|SpawnEmitteratLocation "/Game/StarterContent/Particles/P_MySmoke.P_MySmoke" (Transformation|GetActorLocation))
    (Actor|DestroyActor)))

(event EventBeginPlay
  (Physics|SetSimulatePhysics (Variables|Default|GetCapsuleComponent) true))

(fn ConstructionScript)

(fn Attack
  (bind _mesh (Variables|Character|GetMesh))
  (bind _returnvalue (Components|SkeletalMesh|GetAnimInstance _mesh))
  (Utilities|IsValid _returnvalue
    (:Is%20Valid
      (bind _returnvalue_2 (Animation|Montage|MontagePlay _returnvalue "/Game/Blueprints/Enemies/AM_Attack.AM_Attack" 1.0 "MontageLength" 0.0 true))
      (return _returnvalue_2))))

(fn DamagePlayer
  (Audio|PlaySoundatLocation (.OutItem (Utilities|Array|Random (Variables|Default|GetSwordSounds))) (Transformation|GetActorLocation) "0, 0, 0" 1.0 1.0 0.0 0 0 0 0))

(fn ThrowGranadeAnim
  (bind _returnvalue (Animation|PlayAnimMontage "/Game/Blueprints/Enemies/AM_Throw.AM_Throw" 1.0 "None"))
  (return (+ _returnvalue 2.0)))

(fn SpawnGranade
  (bind _returnvalue (Game|SpawnActorfromClass "/Game/Blueprints/Enemies/EnemyProjectile/BP_EnemyProjectile.BP_EnemyProjectile_C" (Transformation|GetActorTransform) "Undefined" 0 0))
  (Variables|/Script/Engine.MovementComponent|SetVelocity (Variables|/Game/Blueprints/Enemies/EnemyProjectile/BP_EnemyProjectile.BP_EnemyProjectile_C|GetProjectileMovement _returnvalue) (* (Math|Vector|Normalize (+ (- (Transformation|GetActorLocation (Game|Player|GetPlayerPawn 0)) (Transformation|GetActorLocation)) "0,0,50.000000")) 3.5e+03)))