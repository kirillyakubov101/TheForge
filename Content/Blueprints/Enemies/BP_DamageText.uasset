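; Floating damage number actor that displays a Damage value as 3D text above the game world.
; On spawn it writes Damage into a TextRender component and binds to its ActorSequence finishing.
; Each tick it yaws to face the player character.
; When the sequence finishes, the actor destroys itself.
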(event Custom|OnFinished_Event_0
  (Actor|DestroyActor))

(event EventBeginPlay
  (Variables|Default|SetPlayer (Game|GetPlayerCharacter 0))
  (Rendering|Components|TextRender|SetText (Variables|Default|GetTextRender) (Utilities|Text|ToText(Float) (Variables|Default|Getdamage) "HalfToEven"))
  (EventDispatchers|AssignOnFinished (Variables|/Script/ActorSequence.ActorSequenceComponent|GetSequencePlayer (Variables|Default|GetActorSequence)) (delegate Custom|OnFinished_Event_0)))

(event EventTick
  (params (DeltaSeconds :type Float%20%28single-precision%29))
  (Transformation|SetActorRotation (Math|Rotator|MakeRotator 0.0 0.0 (.yaw (Math|Rotator|FindLookatRotation (Transformation|GetActorLocation) (Transformation|GetActorLocation (Variables|Default|GetPlayer)))))))

(fn ConstructionScript)