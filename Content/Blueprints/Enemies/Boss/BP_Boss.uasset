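; Boss enemy that turns to face the player and periodically casts a meteor attack.
; A Tick timer triggers AirAttack, which plays the cast montage, then a meteor spawns above the player's current position halfway through the montage.
; BeginPlay runs a per-frame Delay loop for yaw tracking, while capsule contact damages the player on a cooldown.
; Incoming damage spawns damage text and lowers Health, calling OnBossDeath before destruction at zero.
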(event OnComponentHit(Capsule)
  (params (HitComponent :type Primitive%20Component%20Object%20Reference) (OtherActor :type Actor%20Object%20Reference) (OtherComp :type Primitive%20Component%20Object%20Reference) (NormalImpulse :type Vector :default "0, 0, 0") (Hit :type Hit%20Result%20Structure%20%28by%20ref%29))
  (bind _player (Variables|Default|GetPlayer))
  (if (== OtherActor _player)
    (Utilities|FlowControl|DoOnce false :!label _label
      (:Completed
        (Game|Damage|ApplyDamage _player 5e+01 0 0)
        (Utilities|FlowControl|Delay 2.0)
        (goto _label Reset)))))

(event EventBeginPlay
  (bind _asbp_my_fps (Utilities|Casting|CastToBP_MyFPS (Game|GetPlayerCharacter 0)))
  (Variables|Default|SetPlayer _asbp_my_fps)
  (Transformation|SetActorRotation (Math|Rotator|MakeRotator 0.0 0.0 (.yaw (Math|Rotator|MakeRotfromX (Math|Vector|Normalize (- (Transformation|GetActorLocation (Variables|Default|GetPlayer)) (Transformation|GetActorLocation)))))) :!label _label)
  (Utilities|FlowControl|Delay (Utilities|Time|GetWorldDeltaSeconds))
  (goto _label))

(event EventTick
  (params (DeltaSeconds :type Float%20%28single-precision%29))
  (bind _player (Variables|Default|GetPlayer))
  (bind _returnvalue (Transformation|GetActorLocation _player))
  (bind _output_get (Variables|Default|SetAttackTimer (+ DeltaSeconds (Variables|Default|GetAttackTimer))))
  (if (>= _output_get (Variables|Default|GetAttackCD))
    (Variables|Default|SetAttackTimer 0.0)
    (bind _halfduration (CallFunction|AirAttack))
    (Utilities|FlowControl|Delay _halfduration)
    (Game|SpawnActorfromClass "/Game/Blueprints/Enemies/BossProjectile/BP_Meteor.BP_Meteor_C" (Math|Transform|MakeTransform (Math|Vector|MakeVector (.x _returnvalue) (.y _returnvalue) (Variables|Default|GetMeteorSpawnHeight)) "0, 0, 0" "1.000000,1.000000,1.000000") "Undefined" 0 0)))

(event Game|Damage|EventAnyDamage
  (params (Damage :type Float%20%28single-precision%29) (DamageType :type Damage%20Type%20Object%20Reference) (InstigatedBy :type Controller%20Object%20Reference) (DamageCauser :type Actor%20Object%20Reference))
  (Game|SpawnActorfromClass "/Game/Blueprints/Enemies/BP_DamageText.BP_DamageText_C" (Math|Transform|MakeTransform (Transformation|GetWorldLocation (Variables|Default|GetDamageTextTransform)) "0, 0, 0" "1.000000,1.000000,1.000000") "Undefined" 0 Damage 0)
  (Variables|Default|SetHealth (- (Variables|Default|GetHealth) Damage))
  (if (<= (Variables|Default|GetHealth) 0.0)
    (Default|CallOnBossDeath)
    (Actor|DestroyActor)))

(fn ConstructionScript)

(fn AirAttack
  (bind _skeletalmesh (Variables|Default|GetSkeletalMesh))
  (bind _returnvalue (Components|SkeletalMesh|GetAnimInstance _skeletalmesh))
  (bind _asab_boss_anim (Utilities|Casting|CastToAB_BossAnim _returnvalue))
  (Utilities|IsValid _asab_boss_anim
    (:Is%20Valid
      (bind _returnvalue_2 (Animation|Montage|MontagePlay _returnvalue "/Game/Blueprints/Enemies/Boss/AM_CastSpell.AM_CastSpell" 1.0 "MontageLength" 0.0 true))
      (return (/ _returnvalue_2 2.0)))))