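; BP_BossSpawner stages the boss's entrance and spawns BP_Boss when its SpawnBoss event is called.
; It plays an entrance sound, emits smoke and sparks at SmokePoint, and shakes the BP_MyFPS player's camera.
; After a delay, it triggers an explosion, spawns the boss there, passes it to CallDisplayBossUI, and removes the sparks emitter.
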(event Custom|SpawnBoss
  (bind _smoke_point (Variables|Default|GetSmoke%20Point))
  (bind _smoke_point_2 (Variables|Default|GetSmoke%20Point))
  (bind _returnvalue (Transformation|GetWorldLocation _smoke_point_2))
  (bind _returnvalue_2 (Transformation|GetWorldLocation _smoke_point))
  (Audio|PlaySound2D "/Game/Sounds/SC_BossENTER.SC_BossENTER" 1.0 1.0 0.0 0 0)
  (Effects|SpawnEmitteratLocation "/Game/StarterContent/Particles/P_Smoke.P_Smoke" _returnvalue_2 "0, 0, 0" "15.000000,15.000000,15.000000")
  (bind _returnvalue_3 (Effects|SpawnEmitteratLocation "/Game/StarterContent/Particles/P_Sparks.P_Sparks" _returnvalue_2 "0, 0, 0" "15.000000,15.000000,15.000000"))
  (bind _asbp_my_fps (Utilities|Casting|CastToBP_MyFPS (Game|GetPlayerCharacter 0)))
  (Default|ShakePlayerCamera _asbp_my_fps)
  (Utilities|FlowControl|Delay 4.8)
  (Effects|SpawnEmitteratLocation "/Game/StarterContent/Particles/P_Explosion.P_Explosion" _returnvalue "0, 0, 0" "15.000000,15.000000,15.000000")
  (bind _returnvalue_4 (Game|SpawnActorfromClass "/Game/Blueprints/Enemies/Boss/BP_Boss.BP_Boss_C" (Math|Transform|MakeTransform _returnvalue "0, 0, 0" "1.000000,1.000000,1.000000") "Undefined" 0 0))
  (Default|CallDisplayBossUI _returnvalue_4)
  (Components|DestroyComponent _returnvalue_3))

(fn ConstructionScript)