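; First-person player character Blueprint that adds shooting, dashing, damage feedback and death handling on top of C++ logic.
; Shooting uses a cooldown-gated line trace, dealing random damage to enemies or the boss and spawning explosion effects.
; Dashing launches the character upward, then along its velocity, with a timeline FOV kick.
; Hits trigger a hop and camera shake, while lava contact or lethal damage leads to delayed death.
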(event OnComponentBeginOverlap(LavaDetector)
  (params (OverlappedComponent :type Primitive%20Component%20Object%20Reference) (OtherActor :type Actor%20Object%20Reference) (OtherComp :type Primitive%20Component%20Object%20Reference) (OtherBodyIndex :type Integer) (bFromSweep :type Boolean) (SweepResult :type Hit%20Result%20Structure%20%28by%20ref%29))
  ;[1 0.2285 0.2584] Lava Detection
  (Utilities|FlowControl|Delay 0.5)
  (CallFunction|PlayDeathSound)
  (Utilities|FlowControl|Delay 0.5)
  (Class|MyFPSCharacter|Death))

(event Custom|FOVLerp
  (bind _camera (Variables|Default|GetCamera))
  ;[1 1 1] FOV WHILE DASH
  (bind _value (Timeline|Timeline_0 PlayFromStart)
    (:Update
      (Camera|SetFieldOfView _camera (Math|Float|Lerp 9e+01 1e+02 _value)))
    (:Finished
      (Utilities|FlowControl|Delay 0.1)
      (bind _value_2 (Timeline|Timeline_1 PlayFromStart)
        (:Update
          (Camera|SetFieldOfView _camera (Math|Float|Lerp 1e+02 9e+01 _value_2)))))))

(event EventShoot
  (bind _randdamage (CallFunction|RandomDamage))
  ;[0.5198 1 0.6751] Shooting
  (|CallParentFunction)
  (Utilities|FlowControl|DoOnce false :!label _label
    (:Completed
      (Audio|SpawnSound2D "/Game/Sounds/SC_Blaster.SC_Blaster" 1.0 1.0 0.0 0)
      (bind (_hitactor _impactpoint) (Class|MyFPSCharacter|LineTraceShooting))
      (bind _asbp_enemy (Utilities|Casting|CastToBP_Enemy _hitactor)
        (:then
          (Game|Damage|ApplyDamage _asbp_enemy _randdamage 0 0))
        (:CastFailed
          (bind _asbp_boss (Utilities|Casting|CastToBP_Boss _hitactor)
            (:then
              (Game|Damage|ApplyDamage _asbp_boss _randdamage 0 0))
            (:CastFailed
              _))))
      (Effects|SpawnEmitteratLocation "/Game/StarterContent/Particles/P_Explosion.P_Explosion" _impactpoint "0, 0, 0" "0.800000,0.800000,0.800000" true "AutoRelease")
      (Effects|SpawnEmitteratLocation "/Game/StarterContent/Particles/P_Explosion.P_Explosion" (Transformation|GetWorldLocation (Variables|Default|GetShoot%20Point)) "0, 0, 0" "0.300000,0.300000,0.300000" true "AutoRelease")
      (Utilities|FlowControl|Delay (Variables|Default|GetShootCd))
      (goto _label Reset))))

(event EventDamage
  ;[1 1 1] Damage Dealing
  (Audio|PlaySoundatLocation "/Game/Sounds/SC_GetHit.SC_GetHit" (Transformation|GetActorLocation) "0, 0, 0" 1.0 1.0 0.5 0 0 0 0)
  (if (Class|MyFPSCharacter|IsPlayerDead)
    (Utilities|FlowControl|DoOnce false
      (:Completed
        (Utilities|FlowControl|Delay 0.8)
        (CallFunction|PlayDeathSound)
        (Utilities|FlowControl|Delay 0.5)
        (Class|MyFPSCharacter|Death)))
    (else
      (Character|LaunchCharacter "0, 0,110.000000" false false)
      (Utilities|FlowControl|Delay 0.1)
      (Character|LaunchCharacter "0, 0, 0" false false)
      (Camera|PlayWorldCameraShake "/Game/Blueprints/BP_CameraShake.BP_CameraShake_C" (Transformation|GetActorLocation) 0.0 5e+02))))

(event EventDashEvent
  (bind (_outvelocity _returnvalue) (Class|MyFPSCharacter|CanDash))
  ;[1 1 1] Dashing
  (|CallParentFunction)
  (if _returnvalue
    (Utilities|FlowControl|DoOnce false :!label _label
      (:Completed
        (Audio|PlaySound2D "/Game/Sounds/SC_Dash.SC_Dash" 3.0 1.0 0.0 0 0)
        (Character|LaunchCharacter (Math|Vector|MakeVector 0.0 0.0 (Variables|Default|GetLaunch_Z_Force)) false false)
        (Utilities|FlowControl|Delay 0.1)
        (Character|LaunchCharacter (* (Math|Vector|Normalize _outvelocity) (Variables|Default|GetLaunch_Z_ForceMultiplier)) false false)
        (CallFunction|FOVLerp)
        (Utilities|FlowControl|Delay 0.7)
        (goto _label Reset)))))

(event Input|ActionEvents|InputActionQuitGame
  (params (Key :type Key%20Structure :default "None"))
  ;[1 1 1] Quit
  (:Released
    (Game|QuitGame 0 "Quit" false)))

(fn ConstructionScript)

(fn HealPLayer
  (Default|CallOnGetHealed)
  (Audio|PlaySound2D "/Game/Sounds/SC_Heal.SC_Heal" 1.0 1.0 0.0 0 0)
  (Variables|Default|SetHealthPoints (Variables|Default|GetMaxHealth)))

(fn PlayDeathSound
  (Audio|PlaySound2D "/Game/Sounds/SC_Death.SC_Death" 1.0 1.0 0.0 0 0))

(fn ShakePlayerCamera
  (Camera|PlayWorldCameraShake "/Game/Blueprints/BP_BossArriveCameraShake.BP_BossArriveCameraShake_C" (Transformation|GetActorLocation) 0.0 5e+02 3.0))

(fn RandomDamage
  (return (Math|Conversions|ToFloat(Integer) (Math|Float|Floor (Math|Random|RandomFloatinRange 15.0 35.0)))))

(fn CanDashTest
  (bind _charactermovement (Variables|Character|GetCharacterMovement))
  (bind _velocity (Variables|/Script/Engine.MovementComponent|GetVelocity _charactermovement))
  (return _velocity (and (> (Math|Vector|VectorLength _velocity) 0.0) (not (AI|Components|NavMovement|IsFalling _charactermovement)))))